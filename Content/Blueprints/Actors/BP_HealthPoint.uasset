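; BP_HealthPoint is an interactable spawner actor that emits a stream of pickup cubes.
; OnInteract1 starts a looping 0.1-second timer, and OnInteract2 clears it if the handle is valid.
; Each tick of the timer calls SpawnHealthCube, which spawns a cube at a random horizontal offset around the actor.
; Despite the health naming, the spawned class is BP_ManaCube.
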(event `self.OnInteract1`
  (bind _returnvalue (`KismetSystemLibrary.K2_SetTimerDelegate` (delegate `SpawnHealthCube`) 0.1 true false 0.5))
  (set `self.Timer` _returnvalue))

(event `SpawnHealthCube`
  (bind (_returnvalue_location _returnvalue_rotation _returnvalue_scale) (`KismetMathLibrary.BreakTransform` (`self.GetTransform`)))
  (`|SpawnActorFromClass` "/Game/Blueprints/Actors/BP_ManaCube.BP_ManaCube_C" (`KismetMathLibrary.MakeTransform` (+ _returnvalue_location (`KismetMathLibrary.MakeVector` (* (- (`KismetMathLibrary.RandomFloat`) 0.5) 100.0) (* (- (`KismetMathLibrary.RandomFloat`) 0.5) 100.0))) _returnvalue_rotation _returnvalue_scale) "AdjustIfPossibleButAlwaysSpawn" "MultiplyWithRoot" null null))

(event `self.OnInteract2`
  (bind _timer (`self.Timer`))
  (if (`KismetSystemLibrary.K2_IsValidTimerHandle` _timer)
    (`KismetSystemLibrary.K2_ClearAndInvalidateTimerHandle` _timer)))

(fn `UserConstructionScript`)