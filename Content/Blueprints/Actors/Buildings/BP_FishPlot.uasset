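; BP_FishPlot is an interactable fishing spot that opens the fishing UI and starts fishing for the player's character.
; On interaction, it toggles the fishing widget through the SntpHUD for any option, but calls StartFishing on the character's FishingComponent only for the "Fish" option.
; It then binds to the component's success and closed callbacks, both of which toggle the widget again to dismiss it.
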(event `self.Blueprint_Interact`
  (params (Interactor :type "Actor Object Reference") (OptionName :type Name))
  (bind _asbp_aura_character (cast `/Game/Blueprints/Characters/Aura/BP_AuraCharacter` Interactor))
  (set `self.PlayerCharacter` _asbp_aura_character)
  (`|ExecutionSequence`
    (:`then_0`
      ; Get Param
      (bind _asplayer_controller (cast `PlayerController` (`Pawn.GetController` (`self.PlayerCharacter`))))
      (set `self.PlayerController` _asplayer_controller)
      (bind _assntp_hud (cast `SntpHUD` (`PlayerController.GetHUD` (`self.PlayerController`))))
      (bind _output_get (set `self.HUD` _assntp_hud))
      ; Open Fishing Widget
      (`SntpHUD.ToggleFishingWidget` _output_get (`self.PlayerController`)))
    (:`then_1`
      ; Start Fishing
      (if (== OptionName "Fish")
        (bind _output_get_2 (set `self.FishComponent` (`self.GetComponentByClass` (`self.PlayerCharacter`) "/Script/Sntp.FishingComponent")))
        (`FishingComponent.StartFishing` _output_get_2)))
    (:`then_2`
      ; On Fish Success: Close Fishing Widget
      (add `FishingComponent.OnFishSuccess` (`self.FishComponent`) (delegate `OnFishSuccess_Event`))
      ; Interpret
      (add `FishingComponent.OnFishClosed` (`self.FishComponent`) (delegate `OnFishClosed_Event`)))))

(event `OnFishClosed_Event`
  ; Interpret
  (`SntpHUD.ToggleFishingWidget` (`self.HUD`) (`self.PlayerController`)))

(event `OnFishSuccess_Event`
  ; On Fish Success: Close Fishing Widget
  (`SntpHUD.ToggleFishingWidget` (`self.HUD`) (`self.PlayerController`)))

(fn `UserConstructionScript`)