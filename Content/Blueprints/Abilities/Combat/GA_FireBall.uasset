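; Fireball gameplay ability that turns the avatar toward a target and launches a projectile at it.
; It targets the nearest enemy within a fixed radius, falling back to a point in front of the avatar.
; It updates facing through CombatInterface, then plays the cast montage.
; The Montage.Firebolt gameplay event triggers the projectile spawn and ends the ability, with no handling for montage completion or interruption.
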(event `self.K2_ActivateAbility`
  (bind _returnvalue (`self.GetAvatarActorFromActorInfo`))
  (bind _returnvalue_2 (`SntpAbilitySystemLibrary.GetNearestEnemy` (`self.GetAvatarActorFromActorInfo`) 500.0))
  (`/Engine/EditorBlueprintResources/StandardMacros.IsValid` _returnvalue_2
    (:`Is Valid`
      ;[0.05421 0.15 0.06222 0.5] if get Enemy, hit Enemy
      (set `self.TargetLocation` (`Actor.K2_GetActorLocation` _returnvalue_2)))
    (:`Is Not Valid`
      ;[0.15 0.03964 0.01747 0.5] if None Enemy, hit forward
      (set `self.TargetLocation` (+ (* (`Actor.GetActorForwardVector` _returnvalue) (500.0 500.0 0.0)) (`Actor.K2_GetActorLocation` _returnvalue)))))
  (bind _ascombat_interface (cast `CombatInterface` (`self.GetAvatarActorFromActorInfo`)))
  (`CombatInterface.UpdateFacingTarget` _ascombat_interface (`self.TargetLocation`))
  (`AbilityTask_PlayMontageAndWait.CreatePlayMontageAndWaitProxy` "None" "/Game/Assets/Characters/Wulfa/Animations/AM_Cast_FireBolt_Luoxi.AM_Cast_FireBolt_Luoxi"
    (:`then`
      (`AbilityTask_WaitGameplayEvent.WaitGameplayEvent` (struct :`TagName` "Montage.Firebolt") null true
        (:`EventReceived`
          (`self.SpawnProjectile` (`self.TargetLocation`))
          (`self.K2_EndAbility`))))))