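; Base melee attack gameplay ability that turns the player toward the nearest enemy, or straight ahead, and plays an attack montage.
; It locks move input and combo interruption, then calls a MontageStarted hook for children.
; On authority, gameplay events start and end the ComboComponent hit scan, passing a GE_Damage spec with SetByCaller damage from Attack and fixed resilience.
; Montage completion, interruption or cancellation stops the scan and ends the ability.
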(event `self.K2_ActivateAbility`
  (bind _returnvalue (`self.GetAvatarActorFromActorInfo`))
  (bind _sntpplayercharacter (`self.SntpPlayerCharacter`))
  (bind _returnvalue_2 (`SntpAbilitySystemLibrary.GetNearestEnemy` (`self.GetAvatarActorFromActorInfo`) 500.0))
  (bind _assntp_player_character (cast `SntpPlayerCharacter` (`self.GetAvatarActorFromActorInfo`)))
  (set `self.SntpPlayerCharacter` _assntp_player_character)
  (`/Engine/EditorBlueprintResources/StandardMacros.IsValid` _returnvalue_2
    (:`Is Valid`
      ;[0.05421 0.15 0.06222 0.5] if get Enemy, hit Enemy
      (set `self.TargetLocation` (`Actor.K2_GetActorLocation` _returnvalue_2)))
    (:`Is Not Valid`
      ;[0.15 0.03964 0.01747 0.5] if None Enemy, hit forward
      (set `self.TargetLocation` (+ (* (`Actor.GetActorForwardVector` _returnvalue) (500.0 500.0 0.0)) (`Actor.K2_GetActorLocation` _returnvalue)))))
  (bind _ascombat_interface (cast `CombatInterface` (`self.GetAvatarActorFromActorInfo`)))
  (`CombatInterface.UpdateFacingTarget` _ascombat_interface (`self.TargetLocation`))
  ; Ignore Move Input
  (`SntpPlayerCharacter.SetIgnoreMoveInput` _sntpplayercharacter true)
  (set `ComboComponent.CanInterrupt` false (`SntpPlayerCharacter.GetComboComponent` _sntpplayercharacter))
  (`AbilityTask_PlayMontageAndWait.CreatePlayMontageAndWaitProxy` "None" (`self.AttackMontage`)
    (:`then`
      (`self.MontageStarted`)
      ;[0.3074 1 0.0498 0.5] Hit Scan
      (`self.K2_HasAuthority`
        (:`True`
          (`AbilityTask_WaitGameplayEvent.WaitGameplayEvent` (struct :`TagName` "Event.HitScan.Start") null
            (:`then`
              (`AbilityTask_WaitGameplayEvent.WaitGameplayEvent` (struct :`TagName` "Event.HitScan.End") null
                (:`EventReceived`
                  (`ComboComponent.HitScanEnd` (`SntpPlayerCharacter.GetComboComponent` (`self.SntpPlayerCharacter`))))))
            (:`EventReceived`
              (`self.HandleHitScanStart`))))))
    (:`OnCompleted`
      ;[1 0 0 0.5] End Ability
      (`ComboComponent.HitScanEnd` (`SntpPlayerCharacter.GetComboComponent` (`self.SntpPlayerCharacter`)) :!label _label)
      (`self.K2_EndAbility`))
    (:`OnInterrupted`
      (goto _label))
    (:`OnCancelled`
      (goto _label))))

(event `self.K2_OnEndAbility`
  (params (bWasCancelled :type Boolean)))

(event `MontageStarted`
  ; Override it in child
)

(event `HandleHitScanStart`
  ;[0.3074 1 0.0498 0.5] Handle HitScan Start
  (bind _returnvalue (`AbilitySystemComponent.GetAttributeSet` (`AbilitySystemBlueprintLibrary.GetAbilitySystemComponent` (`self.SntpPlayerCharacter`)) "/Script/Sntp.SntpAttributeSet"))
  (bind (_attack_basevalue _attack_currentvalue) (break `GameplayAttributeData` (`SntpAttributeSet.Attack` _returnvalue)))
  (bind _returnvalue_2 (`AbilitySystemBlueprintLibrary.AssignTagSetByCallerMagnitude` (`self.MakeOutgoingGameplayEffectSpec` "/Game/Blueprints/GameplayEffects/GE_Damage.GE_Damage_C") (struct :`TagName` "Damage") _attack_currentvalue))
  (bind _returnvalue_3 (`AbilitySystemBlueprintLibrary.AssignTagSetByCallerMagnitude` _returnvalue_2 (struct :`TagName` "Resilience") 20.0))
  (`ComboComponent.HitScanStart` (`SntpPlayerCharacter.GetComboComponent` (`self.SntpPlayerCharacter`)) _returnvalue_3))