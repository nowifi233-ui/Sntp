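; BP_AuraCharacter is the Aura player character Blueprint, adding input handling and cosmetic hooks for combat and building.
; Keys slow walking while LeftCtrl is held, cycle and place buildables through BuildManager, and jump by interrupting the combo when ComboComponent and move input allow.
; Events feed a FacingTarget location to Motion Warping and run timelines driving the Dissolve material parameter for weapon spawn and dissolve.
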(event `CombatInterface.UpdateFacingTarget`
  (params (TargetLocation :type "Vector Structure (by ref)"))
  (`MotionWarpingComponent.AddOrUpdateWarpTargetFromLocation` (`self.MotionWarping`) "FacingTarget" TargetLocation))

(event `Key|LeftControl`
  (params (Key :type "Key Structure"))
  (:`Pressed`
    (set `CharacterMovementComponent.MaxWalkSpeed` 300.0 (`self.CharacterMovement`)))
  (:`Released`
    (set `CharacterMovementComponent.MaxWalkSpeed` 600.0 (`self.CharacterMovement`))))

(event `self.StartWeaponDissolveTimeline`
  (params (DynamicMaterialInstance :type "MaterialInstanceDynamic Object Reference"))
  ; Dissolve Weapon Timeline
  (bind (_direction _newtrack_0) (`Timeline|Timeline_0` :!via `PlayFromStart`)
    (:`Update`
      (`MaterialInstanceDynamic.SetScalarParameterValue` DynamicMaterialInstance "Dissolve" _newtrack_0))))

(event `self.StartSpawnWeaponTimeline`
  (params (DynamicMaterialInstance :type "MaterialInstanceDynamic Object Reference"))
  ; Dissolve Weapon Timeline
  (bind (_direction _spawntrack) (`Timeline|Timeline` :!via `PlayFromStart`)
    (:`Update`
      (`MaterialInstanceDynamic.SetScalarParameterValue` DynamicMaterialInstance "Dissolve" _spawntrack))))

(event `Key|E`
  (params (Key :type "Key Structure"))
  (:`Pressed`
    (`BuildableManagerComponent.UpdateCurrentBuildPreviewIndex` (`self.BuildManager`) "Increment")))

(event `Key|Q`
  (params (Key :type "Key Structure"))
  (:`Pressed`
    (`BuildableManagerComponent.UpdateCurrentBuildPreviewIndex` (`self.BuildManager`) "Decrement")))

(event `Key|LeftMouseButton`
  (params (Key :type "Key Structure"))
  (bind _buildmanager (`self.BuildManager`))
  (:`Pressed`
    (`BuildableManagerComponent.TryPlaceBuildable` _buildmanager (`BuildableManagerComponent.CurrentBuildPreviewIndex` _buildmanager))))

(event `Key|SpaceBar`
  (params (Key :type "Key Structure"))
  (:`Pressed`
    (bind _assntp_player_controller (cast `SntpPlayerController` (`self.GetController`)))
    (if (`SntpPlayerController.bIgnoreMoveInput` _assntp_player_controller)
      _
      (elif (`ComboComponent.CanInterrupt` (`self.ComboComponent`))
        (`ComboComponent.Interrupt` (`self.ComboComponent`))
        (`self.Jump`)))))

(fn `UserConstructionScript`)