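; BP_NPCBase is an NPC Blueprint that opens a dialogue when the player interacts with it.
; On interact, it casts the interactor to SntpPlayerCharacter, stores it, and reaches the SntpHUD through that character's player controller.
; It toggles the HUD's dialogue widget with its DialogueComponent, then starts DA_NPC1 on that component.
; Construction, BeginPlay, overlap and Tick contain no logic.
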(event `self.Blueprint_Interact`
  (params (Interactor :type "Actor Object Reference") (OptionName :type Name))
  (`|ExecutionSequence`
    (:`then_0`
      ; Comment
      (bind _assntp_player_character (cast `SntpPlayerCharacter` Interactor))
      (bind _output_get (set `self.SntpPlayerCharacter` _assntp_player_character))
      (bind _asplayer_controller (cast `PlayerController` (`self.GetController` _output_get)))
      (bind _assntp_hud (cast `SntpHUD` (`PlayerController.GetHUD` _asplayer_controller)))
      (`SntpHUD.ToggleDialogueWidget` _assntp_hud _asplayer_controller (`self.DialogueComponent`))
      (`DialogueComponent.StartDialogue` (`self.DialogueComponent`) "/Game/Blueprints/Data/Dialogue/DA_NPC1.DA_NPC1"))))

(fn `UserConstructionScript`)